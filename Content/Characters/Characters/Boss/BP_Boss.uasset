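; BP_Boss is an AI boss character that runs the BT_Boss behavior tree from BeginPlay and shows a lock-on widget when selected.
; Pawn sensing calls DetectPawn against the player pawn, and a DoOnce adds the boss health bar to the viewport.
; Damage reduces health in StatsComp, whose delegates update the bar and, at zero health, call HandleDeath and remove the widget.
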(event `self.ReceiveAnyDamage`
  (params (Damage :type "Float (single-precision)") (DamageType :type "DamageType Object Reference") (InstigatedBy :type "Controller Object Reference") (DamageCauser :type "Actor Object Reference"))
  (`StatsComponent.ReduceHealth` (`self.StatsComp`) Damage))

(event `self.ReceiveBeginPlay`
  (`AIController.RunBehaviorTree` (`AIBlueprintHelperLibrary.GetAIController` self) "/Game/Characters/Characters/Boss/AI/BT_Boss.BT_Boss"))

(event `self.OnSelect`
  (`SceneComponent.SetVisibility` (`self.LockonWidget`) true false))

(event `self.OnDeselect`
  (`SceneComponent.SetVisibility` (`self.LockonWidget`) false true))

(event `self.PawnSensing.OnSeePawn`
  (params (Pawn :type "Pawn Object Reference"))
  (`self.DetectPawn` Pawn (`GameplayStatics.GetPlayerPawn` 0))
  (bind _returnvalue (`|CreateWidget` "/Game/UI/WBP_Boss.WBP_Boss_C"))
  (`/Engine/EditorBlueprintResources/StandardMacros.DoOnce` false
    (:`Completed`
      (bind _output_get (set `self.BossWidget` _returnvalue))
      (`UserWidget.AddToViewport` _output_get 0)
      (`/Game/UI/WBP_Boss.SetHealth` (`self.BossWidget`) (`StatsComponent.GetStatPercentage` (`self.StatsComp`) "Health" "MaxHealth")))))

(event `self.StatsComp.OnHealthPercentUpdateDelegate`
  (params (Percentage :type "Float (single-precision)"))
  (`/Game/UI/WBP_Boss.SetHealth` (`self.BossWidget`) Percentage))

(event `self.StatsComp.OnZeroHealthDelegate`
  (`self.HandleDeath`)
  (`Widget.RemoveFromParent` (`self.BossWidget`)))

(fn `UserConstructionScript`)