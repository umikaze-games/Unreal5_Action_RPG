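; BP_Player is the player character, wiring input, components, animation and HUD together.
; Enhanced Input drives lock-on, combo attacks and sprinting through dedicated components, while attack and sprint delegates drain stamina in StatsComp.
; StatsComp regenerates stamina every tick, takes incoming damage, and pushes percentage updates to the player widget.
; Lock-on target changes feed the anim instance, and zero health shows the death screen and triggers death handling.
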(event `self.ReceiveBeginPlay`
  (bind _returnvalue (`|CreateWidget` "/Game/UI/WBP_Player.WBP_Player_C"))
  (bind _output_get (set `self.PlayerWidget` _returnvalue))
  (`UserWidget.AddToViewport` _output_get 0)
  (`/Game/UI/WBP_Player.SetHealth` (`self.PlayerWidget`) (`StatsComponent.GetStatPercentage` (`self.StatsComp`) "Health" "MaxHealth"))
  (`/Game/UI/WBP_Player.SetStamina` (`self.PlayerWidget`) (`StatsComponent.GetStatPercentage` (`self.StatsComp`) "Stamina" "MaxStamina")))

(event `EnhancedInput|/Game/Input/Acitons/IA_Lockon`
  (params (ActionValue :type Boolean) (ElapsedSeconds :type "Float (double-precision)") (TriggeredSeconds :type "Float (double-precision)") (InputAction :type "InputAction Object Reference" :default "/Game/Input/Acitons/IA_Lockon.IA_Lockon"))
  (:`Started`
    (`LockonComponent.ToggleLockon` (`self.LockonComp`) 750.0)))

(event `self.LockonComp.OnUpdatedTargetDelegate`
  (params (NewTargetActorRef :type "Actor Object Reference"))
  (`PlayerAnimInstance.HandleUpdatedTarget` (`self.PlayerAnim`) NewTargetActorRef))

(event `EnhancedInput|/Game/Input/Acitons/IA_Attack`
  (params (ActionValue :type Boolean) (ElapsedSeconds :type "Float (double-precision)") (TriggeredSeconds :type "Float (double-precision)") (InputAction :type "InputAction Object Reference" :default "/Game/Input/Acitons/IA_Attack.IA_Attack"))
  (:`Started`
    (`CombatComponent.ComboAttack` (`self.CombatComp`))))

(event `self.CombatComp.OnAttackPerformedDelegate`
  (params (Amount :type "Float (single-precision)"))
  (`StatsComponent.ReduceStamina` (`self.StatsComp`) Amount))

(event `EnhancedInput|/Game/Input/Acitons/IA_Sprint`
  (params (ActionValue :type Boolean) (ElapsedSeconds :type "Float (double-precision)") (TriggeredSeconds :type "Float (double-precision)") (InputAction :type "InputAction Object Reference" :default "/Game/Input/Acitons/IA_Sprint.IA_Sprint"))
  (:`Triggered`
    (`PlayerActionsComponent.Sprint` (`self.PlayerActionsComp`)))
  (:`Completed`
    (`PlayerActionsComponent.Walk` (`self.PlayerActionsComp`))))

(event `self.PlayerActionsComp.OnSprintDelegate`
  (params (Cost :type "Float (single-precision)"))
  (`StatsComponent.ReduceStamina` (`self.StatsComp`) Cost))

(event `self.ReceiveTick`
  (params (DeltaSeconds :type "Float (single-precision)"))
  (`StatsComponent.RegenStamina` (`self.StatsComp`)))

(event `self.ReceiveAnyDamage`
  (params (Damage :type "Float (single-precision)") (DamageType :type "DamageType Object Reference") (InstigatedBy :type "Controller Object Reference") (DamageCauser :type "Actor Object Reference"))
  (`StatsComponent.ReduceHealth` (`self.StatsComp`) Damage))

(event `self.StatsComp.OnHealthPercentUpdateDelegate`
  (params (Percentage :type "Float (single-precision)"))
  (`/Game/UI/WBP_Player.SetHealth` (`self.PlayerWidget`) Percentage))

(event `self.StatsComp.OnStaminaPercentUpdateDelegate`
  (params (Percentage :type "Float (single-precision)"))
  (`/Game/UI/WBP_Player.SetStamina` (`self.PlayerWidget`) Percentage))

(event `self.StatsComp.OnZeroHealthDelegate`
  (bind _returnvalue (`|CreateWidget` "/Game/UI/WBP_PlayerDeath.WBP_PlayerDeath_C"))
  (`UserWidget.AddToViewport` _returnvalue 1)
  (`self.HandleDeath`))

(fn `UserConstructionScript`)